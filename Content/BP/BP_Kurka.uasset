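; BP_Kurka is a knife weapon Blueprint that changes its appearance between 2D and 3D states.
; Each tick, In2Dvolume reads the 2Dswitch flag and swaps the mesh material and scale, halving its size in 2D.
; The construction script sets separate 2D and 3D damage values.
; Nodes to choose between them and damage characters hit during the owner's swing are disconnected and never run.
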(event Custom|In2Dvolume
  (bind _staticmesh (Variables|Default|GetStaticMesh))
  (if (Variables|Default|Get2Dswitch)
    (Rendering|Material|SetMaterial _staticmesh 0 "/Game/Material/M_2DWhite.M_2DWhite")
    (Transformation|SetWorldScale3D _staticmesh "0.500000,0.500000,0.500000")
    (else
      (Rendering|Material|SetMaterial _staticmesh 0 "/Game/Material/M_White.M_White")
      (Transformation|SetWorldScale3D _staticmesh "1.000000,1.000000,1.000000"))))

(event EventBeginPlay)

(event Collision|EventActorBeginOverlap
  (params (OtherActor :type Actor%20Object%20Reference)))

(event EventTick
  (params (DeltaSeconds :type Float%20%28single-precision%29))
  (CallFunction|In2Dvolume))

(fn ConstructionScript
  (|CallParentFunction)
  (Variables|Default|Set3Ddamage 1e+02)
  (Variables|Default|Set2Ddamage 5e+01))