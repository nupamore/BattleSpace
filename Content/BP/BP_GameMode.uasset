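; Game mode for a networked match on Level_Test that assigns the player a character and tracks a countdown timer.
; On BeginPlay it possesses the BP_Character matching the "id" option (default "red"), optionally connecting to a hardcoded Socket.IO server and binding enemy and rank events.
; Destroying that character spawns and possesses a replacement, rebinds the destroy handler and emits "player respawn".
; Tick derives remaining minutes and seconds from TimeLimit and real time.
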(event Custom|OnDestroyed_event_0
  (params (DestroyedActor :type Actor%20Object%20Reference))
  (bind _returnvalue (Game|SpawnActorfromClass "/Game/BP/Character/BP_Character.BP_Character_C" (Variables|Default|GetRespawnTransform) "Undefined" 0 0))
  (Pawn|Possess (Game|GetPlayerController 0) _returnvalue)
  (CallFunction|Respawn))

(event Custom|GameTimer
  (Variables|Default|SetcurrentTime (Math|Float|Truncate (Utilities|Time|GetRealTimeSeconds)))
  (Variables|Default|SetlimitMinutes (/ (- (Variables|Default|GettimeLimit) (Variables|Default|GetcurrentTime)) 60))
  (Variables|Default|SetlimitSeconds (Math|Integer|%(Integer) (- (Variables|Default|GettimeLimit) (Variables|Default|GetcurrentTime)) 60)))

(event Custom|Respawn
  (bind _asbp_character (Utilities|Casting|CastToBP_Character (Game|GetPlayerCharacter 0)))
  (Game|AssignOnDestroyed _asbp_character (delegate Custom|OnDestroyed_event_0))
  (bind _returnvalue (Class|SIOJsonObject|ConstructJsonObject))
  (Class|SIOJsonObject|SetStringField _returnvalue "id" (Variables|Default|Getid))
  (Class|SocketIOClientComponent|Emit (Variables|Default|GetSocketIOClient) "player respawn" (Class|SIOJLibrary|ToJsonValue(JsonObject) _returnvalue) "/"))

(event EventBeginPlay
  (bind _socketioclient (Variables|Default|GetSocketIOClient))
  (bind _optionsstring (Variables|Default|GetOptionsString))
  (bind _returnvalue (Class|GameplayStatics|ParseOption _optionsstring "id"))
  (bind _returnvalue_2 (Game|GetCurrentLevelName true))
  (if (Utilities|Enum|Equal(Enum) _returnvalue_2 "Level_Test")
    (if (Utilities|Enum|NotEqual(Enum) _returnvalue "")
      (Variables|Default|Setid _returnvalue)
      (else
        (Variables|Default|Setid "red")))
    (bind _outactors (Actor|GetAllActorsOfClass "/Game/BP/Character/BP_Character.BP_Character_C"))
    (for _array_element _outactors
      (if (Utilities|Enum|Equal(Enum) (Variables|/Game/BP/Character/BP_Character.BP_Character_C|Getid _array_element) (Variables|Default|Getid))
        (bind _asbp_character (Utilities|Casting|CastToBP_Character _array_element))
        (Pawn|Possess (Game|GetPlayerController 0) _asbp_character)
        (Utilities|FlowControl|Sequence
          (:then_0
            ;[1 1 1] Connect
            (if (Variables|Default|GettryConnect)
              (Class|SocketIOClientComponent|Connect (Variables|Default|GetSocketIOClient) "http://52.78.202.135:17915")
              (Utilities|Casting|CastToBP_GameMode (Game|GetGameMode))
              (Class|SocketIOClientComponent|Emit _socketioclient "join player" (Class|SIOJLibrary|ToJsonValue(String) (Variables|Default|Getid)) "/")
              (Class|SocketIOClientComponent|BindEvent _socketioclient "enemy controlled" "/")
              (Class|SocketIOClientComponent|BindEvent _socketioclient "enemy respawn" "/")
              (Class|SocketIOClientComponent|BindEvent _socketioclient "enemy status" "/")
              (Class|SocketIOClientComponent|BindEvent _socketioclient "rank" "/")))
          (:then_1
            (bind _asbp_character_2 (Utilities|Casting|CastToBP_Character (Game|GetPlayerCharacter 0)))
            (Game|AssignOnDestroyed _asbp_character_2 (delegate Custom|OnDestroyed_event_0))
            (bind _returnvalue_3 (Class|SIOJsonObject|ConstructJsonObject))
            (Class|SIOJsonObject|SetStringField _returnvalue_3 "id" (Variables|Default|Getid))
            (Class|SocketIOClientComponent|Emit (Variables|Default|GetSocketIOClient) "player respawn" (Class|SIOJLibrary|ToJsonValue(JsonObject) _returnvalue_3) "/")))))))

(event EventTick
  (params (DeltaSeconds :type Float%20%28single-precision%29))
  (CallFunction|GameTimer))

(fn ConstructionScript)