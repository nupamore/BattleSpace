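; BP_2dVolume is a volume that switches overlapping characters, bullets, guns and knives into 2D mode through their 2Dswitch flag, clearing it on exit.
; It tracks overlapping actors in an array and divides bullet velocity by SpeedRatio on entry, multiplying it back on exit.
; A player-controlled character starts a timeline that lerps camera FOV between 90 and 50; exit replays that timeline from the start rather than reversing it.
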(event EventBeginPlay)

(event Collision|EventActorBeginOverlap
  (params (OtherActor :type Actor%20Object%20Reference))
  (Utilities|Array|Add (Variables|Default|GetOverlapActorArray) OtherActor)
  (bind _asbp_character (Utilities|Casting|CastToBP_Character OtherActor)
    (:then
      (Variables|Default|SetplayerCamera (Variables|/Game/BP/Character/BP_Character.BP_Character_C|GetCamera _asbp_character))
      (Variables|/Game/BP/Character/BP_Character.BP_Character_C|Set2Dswitch _asbp_character true)
      (if (Pawn|IsPlayerControlled _asbp_character)
        (bind _fov (Timeline|타임라인_0 PlayFromStart)
          (:Update
            (if (Utilities|IsValid (Variables|Default|GetplayerCamera))
              (Camera|SetFieldOfView (Variables|Default|GetplayerCamera) (Math|Float|Lerp 9e+01 5e+01 _fov)))))))
    (:CastFailed
      (bind _asbp_bullet (Utilities|Casting|CastToBP_Bullet OtherActor)
        (:then
          (Variables|/Game/BP/BP_Bullet.BP_Bullet_C|Set2Dswitch _asbp_bullet true)
          (Variables|/Script/Engine.MovementComponent|SetVelocity (Variables|/Game/BP/BP_Bullet.BP_Bullet_C|GetProjectileMovement _asbp_bullet) (/ (Variables|/Script/Engine.MovementComponent|GetVelocity (Variables|/Game/BP/BP_Bullet.BP_Bullet_C|GetProjectileMovement _asbp_bullet)) (Variables|Default|GetSpeedRatio))))
        (:CastFailed
          (bind _asbp_gun (Utilities|Casting|CastToBP_Gun OtherActor)
            (:then
              (Variables|/Game/BP/BP_Gun.BP_Gun_C|Set2Dswitch _asbp_gun true))
            (:CastFailed
              (bind _asbp_knife (Utilities|Casting|CastToBP_Knife OtherActor))
              (Variables|/Game/BP/BP_Knife.BP_Knife_C|Set2Dswitch _asbp_knife true))))))))

(event Collision|EventActorEndOverlap
  (params (OtherActor :type Actor%20Object%20Reference))
  (bind _playercamera (Variables|Default|GetplayerCamera))
  (bind _overlapactorarray (Variables|Default|GetOverlapActorArray))
  (Utilities|Array|RemoveIndex _overlapactorarray (Utilities|Array|FindItem _overlapactorarray OtherActor))
  (bind _asbp_character (Utilities|Casting|CastToBP_Character OtherActor)
    (:then
      (Variables|/Game/BP/Character/BP_Character.BP_Character_C|Set2Dswitch _asbp_character false)
      (if (Pawn|IsPlayerControlled _asbp_character)
        (bind _fov (Timeline|타임라인_0 PlayFromStart)
          (:Update
            (if (Utilities|IsValid _playercamera)
              (Camera|SetFieldOfView _playercamera (Math|Float|Lerp 9e+01 5e+01 _fov)))))))
    (:CastFailed
      (bind _asbp_bullet (Utilities|Casting|CastToBP_Bullet OtherActor)
        (:then
          (Variables|/Game/BP/BP_Bullet.BP_Bullet_C|Set2Dswitch _asbp_bullet false)
          (Variables|/Script/Engine.MovementComponent|SetVelocity (Variables|/Game/BP/BP_Bullet.BP_Bullet_C|GetProjectileMovement _asbp_bullet) (* (Variables|/Script/Engine.MovementComponent|GetVelocity (Variables|/Game/BP/BP_Bullet.BP_Bullet_C|GetProjectileMovement _asbp_bullet)) (Variables|Default|GetSpeedRatio))))
        (:CastFailed
          (bind _asbp_gun (Utilities|Casting|CastToBP_Gun OtherActor)
            (:then
              (Variables|/Game/BP/BP_Gun.BP_Gun_C|Set2Dswitch _asbp_gun false))
            (:CastFailed
              (bind _asbp_knife (Utilities|Casting|CastToBP_Knife OtherActor))
              (Variables|/Game/BP/BP_Knife.BP_Knife_C|Set2Dswitch _asbp_knife false))))))))

(fn ConstructionScript)