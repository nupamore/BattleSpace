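; Projectile bullet with 2D and 3D modes that damages any BP_Character it hits other than its owner.
; Tick watches 2Dswitch for changes and reapplies the mode's damage, material, collision radius, mesh scale and gravity.
; Character damage requires a root-component hit and destroys the bullet; other sphere impacts destroy it only in 3D mode.
; Overlap events with BP_2dVolume spawn particles but leave the switch untouched.
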(event OnComponentBeginOverlap(Sphere)
  (params (OverlappedComponent :type Primitive%20Component%20Object%20Reference) (OtherActor :type Actor%20Object%20Reference) (OtherComp :type Primitive%20Component%20Object%20Reference) (OtherBodyIndex :type Integer) (bFromSweep :type Boolean) (SweepResult :type Hit%20Result%20Structure%20%28by%20ref%29))
  (Utilities|Casting|CastToBP_2dVolume OtherActor)
  (Effects|SpawnEmitteratLocation "/Game/InfinityBladeEffects/Effects/FX_Ability/Defense/P_Shield_Spawn.P_Shield_Spawn" (Transformation|GetWorldLocation (Variables|Default|GetSphere)) "90.000000, 0,90.000000"))

(event OnComponentHit(Sphere)
  (params (HitComponent :type Primitive%20Component%20Object%20Reference) (OtherActor :type Actor%20Object%20Reference) (OtherComp :type Primitive%20Component%20Object%20Reference) (NormalImpulse :type Vector :default "0, 0, 0") (Hit :type Hit%20Result%20Structure%20%28by%20ref%29))
  (Effects|SpawnEmitteratLocation "/Game/InfinityBladeEffects/Effects/FX_Monsters/FX_Monster_Ausar/P_AU_Shieldslam_Impact.P_AU_Shieldslam_Impact" (Transformation|GetWorldLocation (Variables|Default|GetSphere)) "90.000000, 0,90.000000")
  (if (not (Variables|Default|Get2Dswitch))
    (Actor|DestroyActor)))

(event Custom|In2Dvolume
  (bind _2dswitch (Variables|Default|Get2Dswitch))
  ;[1 1 1] 변수 변화 체크
  (if (Math|Boolean|NotEqual(Boolean) _2dswitch (Variables|Default|Get2DswitchCheck))
    (Variables|Default|Set2DswitchCheck _2dswitch)
    (CallFunction|SetOptioninVolume)))

(event Custom|SetOptionInVolume
  (bind _projectilemovement (Variables|Default|GetProjectileMovement))
  (bind _staticmesh (Variables|Default|GetStaticMesh))
  (bind _sphere (Variables|Default|GetSphere))
  (bind _staticmesh_2 (Variables|Default|GetStaticMesh))
  ;[1 1 1] setOptionInVolume
  (if (Variables|Default|Get2Dswitch)
    (Variables|Default|SetbulletDamage (Variables|Default|Get2Ddamage))
    (Rendering|Material|SetMaterial _staticmesh 0 "/Game/Material/M_2DWhite.M_2DWhite")
    (Components|Sphere|SetSphereRadius _sphere 1e+01 true)
    (Transformation|SetWorldScale3D _staticmesh_2 "10.000000,20.000000,20.000000")
    (Variables|/Script/Engine.ProjectileMovementComponent|SetProjectileGravityScale _projectilemovement 1.0)
    (else
      (Variables|Default|SetbulletDamage (Variables|Default|Get3Ddamage))
      (Rendering|Material|SetMaterial _staticmesh 0 "/Game/Material/M_Light.M_Light")
      (Components|Sphere|SetSphereRadius _sphere 1.0 true)
      (Transformation|SetWorldScale3D _staticmesh_2 "1.000000,1.000000,1.000000")
      (Variables|/Script/Engine.ProjectileMovementComponent|SetProjectileGravityScale _projectilemovement 0.5))))

(event EventBeginPlay
  (CallFunction|SetOptioninVolume)
  (Audio|PlaySound2D "/Game/FirstPerson/Audio/FirstPersonTemplateWeaponFire02.FirstPersonTemplateWeaponFire02"))

(event EventTick
  (params (DeltaSeconds :type Float%20%28single-precision%29))
  (CallFunction|In2Dvolume))

(event Collision|EventHit
  (params (MyComp :type Primitive%20Component%20Object%20Reference) (Other :type Actor%20Object%20Reference) (OtherComp :type Primitive%20Component%20Object%20Reference) (bSelfMoved :type Boolean) (HitLocation :type Vector) (HitNormal :type Vector :default "0, 0, 0") (NormalImpulse :type Vector :default "0, 0, 0") (Hit :type Hit%20Result%20Structure%20%28by%20ref%29))
  (bind _returnvalue (VehicleSound|GetRootComponent Other))
  (if (Utilities|IsValid Other)
    (if (!= Other (Variables|Default|GetbulletOwner))
      (if (== OtherComp _returnvalue)
        (bind _asbp_character (Utilities|Casting|CastToBP_Character Other))
        (Default|GetDamage _asbp_character (Variables|Default|GetbulletDamage))
        (Default|AttackedUI _asbp_character)
        (Effects|SpawnEmitteratLocation "/Game/InfinityBladeEffects/Effects/FX_Ability/Defense/P_Shield_Spawn.P_Shield_Spawn" HitLocation)
        (Development|PrintString (Utilities|GetDisplayName _returnvalue))
        (Actor|DestroyActor)))))

(event Collision|EventActorEndOverlap
  (params (OtherActor :type Actor%20Object%20Reference))
  (Utilities|Casting|CastToBP_2dVolume (stale OnComponentBeginOverlap(Sphere) OtherActor))
  (Effects|SpawnEmitteratLocation "/Game/InfinityBladeEffects/Effects/FX_Ability/Defense/P_Shield_Spawn.P_Shield_Spawn" (Transformation|GetWorldLocation (Variables|Default|GetSphere)) "90.000000, 0,90.000000"))

(fn ConstructionScript)